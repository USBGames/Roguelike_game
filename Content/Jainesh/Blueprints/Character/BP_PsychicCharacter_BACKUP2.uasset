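; Psychic character Blueprint, named as a backup, with procedural first-person motion on an offset root.
; Jumping and landing play a timeline-driven dip that lowers FPOffsetRoot, with landing strength scaled by vertical speed.
; Walk bob, velocity lag, in-air tilt and look-based sway are computed in a Walking timeline and two helper functions, but that timeline is unconnected.
; Most of those computed values are only stored, not applied here.
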(event Custom|Dip
  (params (Speed :type Float%20%28double-precision%29) (Strength :type Float%20%28double-precision%29))
  (bind _fpoffsetroot (Variables|Default|GetFPOffsetRoot))
  (bind _relativelocation (Variables|/Script/Engine.SceneComponent|GetRelativeLocation _fpoffsetroot))
  ;[1 1 1] Set DIP Parameters
  (Components|Timeline|SetPlayRate (Variables|Default|GetDIp_TL) Speed)
  (Variables|Default|SetDipStrength Strength)
  ;[1 1 1] Update DIP Alpha
  (bind _dip_alpha (Timeline|DIp_TL PlayFromStart)
    (:Update
      (Variables|Default|SetDipAlpha (* _dip_alpha (Variables|Default|GetDipStrength)))
      ;[1 1 1] Update FPRootOffset
      (Transformation|SetRelativeLocation (Variables|Default|GetFPOffsetRoot) (Math|Vector|MakeVector (.x _relativelocation) (.y _relativelocation) (Math|Float|Lerp 0.0 -1e+01 (Variables|Default|GetDipAlpha))) false false))))

(event Custom|LandingDip
  (bind _charactermovement (Variables|Character|GetCharacterMovement))
  ;[1 1 1] Landing Dip
  (CallFunction|Dip 2.0 (Math|Float|Clamp(Float) (Math|Float|NormalizetoRange (Math|Vector|VectorLength (Math|Vector|MakeVector 0.0 0.0 (.z (Pawn|Components|CharacterMovement|GetLastUpdateVelocity _charactermovement)))) 0.0 (Variables|/Script/Engine.CharacterMovementComponent|GetJumpZVelocity _charactermovement)) 0.0 0.7)))

(event Custom|OnJumped_1
  (CallFunction|Dip 2.0 0.7))

(event Custom|OnLanded_1
  (params (Hit :type Hit%20Result%20Structure%20%28by%20ref%29))
  (CallFunction|LandingDip))

(event EventBeginPlay)

(event Collision|EventActorBeginOverlap
  (params (OtherActor :type Actor%20Object%20Reference)))

(event EventTick
  (params (DeltaSeconds :type Float%20%28single-precision%29)))

(fn ConstructionScript)

(fn GetVelocityVars
  (bind _returnvalue (Transformation|GetVelocity))
  (bind _returnvalue_2 (Utilities|Time|GetWorldDeltaSeconds))
  (bind _returnvalue_3 (Utilities|Time|GetWorldDeltaSeconds))
  (bind _basewalkspeed (Variables|Default|GetBaseWalkSpeed))
  (bind _returnvalue_4 (/ _returnvalue_3 1.0))
  (bind _returnvalue_5 (/ _returnvalue_4 12.0))
  (bind _output_get (Variables|Default|SetLocationLagPos (Math|Interpolation|VInterpTo (Variables|Default|GetLocationLagPos) (Math|Vector|ClampVectorSize (* (Math|Vector|MakeVector (/ (Math|Vector|DotProduct _returnvalue (Transformation|GetActorRightVector)) _basewalkspeed) (/ (Math|Vector|DotProduct _returnvalue (Transformation|GetActorForwardVector)) (* _basewalkspeed -1.0)) (/ (Math|Vector|DotProduct _returnvalue (Transformation|GetActorUpVector)) (* (Variables|/Script/Engine.CharacterMovementComponent|GetJumpZVelocity (Variables|Character|GetCharacterMovement)) -1.0))) 2.0) 0.0 4.0) _returnvalue_2 (/ (/ 1.0 _returnvalue_2) 6.0))))
  (Variables|Default|SetInAirTilt (Math|Interpolation|RInterpTo (Variables|Default|GetInAirTilt) (Math|Rotator|MakeRotator 0.0 (* (.z _output_get) -2.0) 0.0) _returnvalue_3 _returnvalue_5))
  (Variables|Default|SetInAirOffset (Math|Interpolation|VInterpTo (Variables|Default|GetInAirOffset) (Math|Vector|MakeVector (* (.z _output_get) -0.5) 0.0 0.0) _returnvalue_3 _returnvalue_5)))

(fn GetLookInputVars
  (params (CamRotPrev :type Rotator))
  (bind _returnvalue (Pawn|GetControlRotation :!class /Script/Engine.Pawn))
  (bind _returnvalue_2 (Transformation|GetActorRotation))
  (bind _returnvalue_3 (Utilities|Time|GetWorldDeltaSeconds))
  (bind _fpoffsetroot (Variables|Default|GetFPOffsetRoot))
  (bind _returnvalue_4 (Math|Rotator|Delta(Rotator) _returnvalue _returnvalue_2))
  (bind _relativelocation (Variables|/Script/Engine.SceneComponent|GetRelativeLocation _fpoffsetroot))
  (bind _returnvalue_5 (Math|Float|NormalizetoRange (.pitch _returnvalue_4) -9e+01 9e+01))
  (Utilities|FlowControl|Sequence
    (:then_0
      ;[1 1 1] Pitch Offset
      (Variables|Default|SetPitchOffsetPos (Math|Vector|MakeVector 0.0 (Math|Float|Lerp 3.0 -3.0 _returnvalue_5) (Math|Float|Lerp 2.0 -2.0 _returnvalue_5)))
      (Transformation|SetRelativeLocation _fpoffsetroot (Math|Vector|MakeVector (Math|Float|Lerp 5.0 0.0 (Math|Float|Clamp(Float) (Math|Float|NormalizetoRange _returnvalue_5 0.0 0.5))) (.y _relativelocation) (.z _relativelocation)) false false))
    (:then_1
      ;[1 1 1] Camera Rotation Rate
      (bind _output_get (Variables|Default|SetCamRotCurrent (Transformation|GetWorldRotation (Variables|Default|GetCameraComponent))))
      (Variables|Default|SetCamRotRate (Math|Interpolation|RInterpTo (Variables|Default|GetCamRotRate) (Math|Rotator|MakeRotator (Math|Float|Clamp(Float) (* (.Pitch (Math|Rotator|BreakRotator (Math|Rotator|Delta(Rotator) _output_get CamRotPrev))) -1.0) -5.0 5.0) 0.0 (Math|Float|Clamp(Float) (.Yaw (Math|Rotator|BreakRotator (Math|Rotator|Delta(Rotator) _output_get CamRotPrev))) -5.0 5.0)) _returnvalue_3 (/ (/ _returnvalue_3 1.0) 1e+02))))
    (:then_2
      ;[1 1 1] Camera Rotation Offset
      (Variables|Default|SetCamRotOffset (Math|Vector|MakeVector (Math|Float|Lerp -6.0 6.0 (Math|Float|NormalizetoRange (.yaw (Variables|Default|GetCamRotRate)) -5.0 5.0)) 0.0 (Math|Float|Lerp -1e+01 1e+01 (Math|Float|NormalizetoRange (.roll (Variables|Default|GetCamRotRate)) -5.0 5.0)))))))